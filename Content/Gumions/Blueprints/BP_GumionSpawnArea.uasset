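; BP_GumionSpawnArea is a spawn volume that populates its bounds with BP_Gumion actors at random intervals.
; On BeginPlay, TimerEvent spawns one at a random point in the bounds with an incrementing Index, then re-arms itself with a random delay.
; The loop runs while the world's BP_Gumion count is at most MaxEnemigos, then stops without restarting.
; The Spawn function is an empty stub.
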(event `self.ReceiveBeginPlay`
  (`self.TimerEvent`))

(event `self.ReceiveTick`
  (params (DeltaSeconds :type "Float (single-precision)")))

(event `TimerEvent`
  (bind _outactors (`GameplayStatics.GetAllActorsOfClass` "/Game/Gumions/Characters/BP_Gumion.BP_Gumion_C"))
  (if (<= (`KismetArrayLibrary.Array_Length` _outactors) (`self.MaxEnemigos`))
    (`self.SpawnCharacter`)
    (`KismetSystemLibrary.K2_SetTimerDelegate` (delegate `TimerEvent`) (+ (* (`KismetMathLibrary.RandomFloat`) 5.0) 1.0))))

(event `SpawnCharacter`
  (bind (_origin _boxextent) (`self.GetActorBounds` self false))
  (bind _output_get (set `self.counter` (+ (`self.counter`) 1)))
  (`|SpawnActorFromClass` "/Game/Gumions/Characters/BP_Gumion.BP_Gumion_C" (`KismetMathLibrary.MakeTransform` (`KismetMathLibrary.RandomPointInBoundingBox` _origin _boxextent)) "Undefined" "OverrideRootScale" null _output_get null))

(fn `Spawn`)

(fn `UserConstructionScript`)