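; BP_Gumion is an AI creature that keeps moving toward the player controller, hopping at random and merging with other Gumions.
; On collision, the larger one, or higher Index on a tie, absorbs the other's Tamano and grows by timeline while the other shrinks away.
; Tick counts frames without horizontal movement to trigger a stronger unstuck jump; the counter never resets.
; Crush (Aplastar) and hand-overlap reactions are unwired stubs.
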(event `self.ReceiveTick`
  (params (DeltaSeconds :type "Float (single-precision)"))
  (bind _returnvalue (* (`SceneComponent.K2_GetComponentLocation` (`self.RootComponent`)) (1.0 1.0 0.0)))
  (if (== _returnvalue (`self.saveStuckPosition`))
    (bind _result (`/Engine/EditorBlueprintResources/StandardMacros.IncrementInt` (`self.saveStuckCounter`))
      (:`  `
        (if (>= _result 500)
          (`self.Unstuck`))))
    (else
      (set `self.saveStuckPosition` _returnvalue))))

(event `self.ReceiveBeginPlay`
  (`self.BuscaAlJugador`)
  (`self.SaltaAleatorio`))

(event `SaltaAleatorio`
  (if (== (`KismetMathLibrary.RandomInteger` 5) 0)
    (`self.Jump`))
  (`KismetSystemLibrary.K2_SetTimerDelegate` (delegate `SaltaAleatorio`) (+ (`KismetMathLibrary.RandomFloat`) 1.0)))

(event `Unstuck`
  (set `CharacterMovementComponent.JumpZVelocity` 800.0 (`self.CharacterMovement`))
  (`self.Jump`))

(event `self.ReceiveActorBeginOverlap`
  (params (OtherActor :type "Actor Object Reference")))

(event `VeAlCentro`
  (`|AIMoveTo` null (0.0 0.0 0.0) null
    (:`OnSuccess`
      _)
    (:`OnFail`
      _))
  (`self.BuscaAlJugador` :!label _label))

(event `BuscaAlJugador`
  (`|AIMoveTo` self (0.0 0.0 0.0) (`GameplayStatics.GetPlayerController` 0)
    (:`OnSuccess`
      (goto _label))
    (:`OnFail`
      (goto _label))))

(event `self.ReceiveHit`
  (params (MyComp :type "PrimitiveComponent Object Reference") (Other :type "Actor Object Reference") (OtherComp :type "PrimitiveComponent Object Reference") (bSelfMoved :type Boolean) (HitLocation :type "Vector Structure") (HitNormal :type "Vector Structure") (NormalImpulse :type "Vector Structure") (Hit :type "HitResult Structure (by ref)"))
  (bind _tamano (`self.Tamano`))
  (if (== (`GameplayStatics.GetObjectClass` Other) (`GameplayStatics.GetObjectClass` self))
    (bind _asbp_gumion (cast `/Game/Gumions/Characters/BP_Gumion` Other))
    (bind _tamano_2 (`/Game/Gumions/Characters/BP_Gumion.Tamano` _asbp_gumion))
    (if (or (> _tamano _tamano_2) (and (== _tamano _tamano_2) (> (`self.index`) (`/Game/Gumions/Characters/BP_Gumion.index` _asbp_gumion))))
      (set `self.lastTamano` _tamano)
      (set `self.Tamano` (+ _tamano _tamano_2))
      (`self.PreDestroyActor` _asbp_gumion)
      (`self.Crecer`))))

(event `PreDestroyActor`
  (`PrimitiveComponent.SetCollisionEnabled` (`self.CapsuleComponent`) "NoCollision")
  (`NavMovementComponent.StopActiveMovement` (`self.CharacterMovement`))
  (bind (_direction _newtrack_0) (`Timeline|Desapareciendo` :!via `PlayFromStart`)
    (:`Update`
      (`self.SetActorScale3D` (* (* (1.0 1.0 1.0) (`self.Tamano`)) _newtrack_0)))
    (:`Finished`
      (`self.K2_DestroyActor`))))

(event `Crecer`
  (`PrimitiveComponent.SetCollisionEnabled` (`self.CapsuleComponent`) "NoCollision")
  (`NavMovementComponent.StopActiveMovement` (`self.CharacterMovement`))
  (bind _escala (`self.GetEscala` (`self.Tamano`)))
  (bind _escala_2 (`self.GetEscala` (`self.lastTamano`)))
  (bind (_direction _newtrack_0) (`Timeline|Creciendo` :!via `PlayFromStart`)
    (:`Update`
      (`self.SetActorScale3D` (+ _escala_2 (* (- _escala _escala_2) _newtrack_0))))
    (:`Finished`
      (`PrimitiveComponent.SetCollisionEnabled` (`self.CapsuleComponent`) "QueryAndPhysics"))))

(event `Aplastar`)

(event `self.Box.OnComponentBeginOverlap`
  (params (OverlappedComponent :type "PrimitiveComponent Object Reference") (OtherActor :type "Actor Object Reference") (OtherComp :type "PrimitiveComponent Object Reference") (OtherBodyIndex :type Integer) (bFromSweep :type Boolean) (SweepResult :type "HitResult Structure (by ref)"))
  (bind _returnvalue (`KismetSystemLibrary.GetObjectName` OtherActor))
  (if (or (`KismetStringLibrary.EqualEqual_StrStr` _returnvalue "LeftHand") (`KismetStringLibrary.EqualEqual_StrStr` _returnvalue "RightHand") (== (`GameplayStatics.GetObjectClass` OtherActor) "/Game/ThirdPersonBP/Blueprints/ThirdPersonCharacter.ThirdPersonCharacter_C"))
    _))

(fn `GetEscala`
  (params (tamano :type "Float (double-precision)"))
  (returns (Escala :type "Vector Structure"))
  (return (+ (* (1.0 1.0 1.0) (/ tamano 2.0)) (0.25 0.25 0.25))))

(fn `UserConstructionScript`
  (locals (NewLocalVar_0 :type "Vector Structure" :default (1.0 1.0 1.0)))
  (bind _escala (`self.GetEscala` (`self.Tamano`)))
  (`self.SetActorScale3D` _escala))